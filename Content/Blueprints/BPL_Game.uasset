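; BPL_Game is a Blueprint function library with shared helpers for player detection and hit knockback.
; FnBPLFindPlayer line-traces on the Camera channel to the player and reports found when it hits the player within the maximum distance, with optional debug drawing.
; FnBPLApplyHitPushback launches a Character away from an origin at a given strength, adding a small upward push and overriding existing velocity.
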(fn FnBPLFindPlayer
  (params (PlayerRef :type Character%20Object%20Reference) (StartLocation :type Vector) (MaxDetectionDistance :type Float%20%28double-precision%29) (Debug :type Boolean))
  (Utilities|IsValid PlayerRef
    (:Is%20Valid
      (Utilities|FlowControl|Sequence
        (:then_0
          (bind _outhit (Collision|LineTraceByChannel 0 StartLocation (Transformation|GetActorLocation PlayerRef) "TraceTypeQuery2" false 0 (select Debug "ForDuration" "None") true "(R=1.000000,G=0.000000,B=0.000000,A=1.000000)" "(R=0.000000,G=1.000000,B=0.000000,A=1.000000)" 0.1))
          (if (and (== (.HitActor (Collision|BreakHitResult _outhit)) PlayerRef) (< (Math|Vector|Distance(Vector) (.TraceStart (Collision|BreakHitResult _outhit)) (.TraceEnd (Collision|BreakHitResult _outhit))) MaxDetectionDistance))
            (LocalVariables|SetPlayerFound true)
            (else
              (LocalVariables|SetPlayerFound false))))
        (:then_1
          (return (LocalVariables|GetPlayerFound)))))
    (:Is%20Not%20Valid
      (return (LocalVariables|GetPlayerFound)))))

(fn FnBPLApplyHitPushback
  (params (ObjectToApplyPushback :type Actor%20Object%20Reference) (PushbackOriginLocation :type Vector) (Strength :type Float%20%28double-precision%29))
  (bind _ascharacter (Utilities|Casting|CastToCharacter ObjectToApplyPushback))
  (Character|LaunchCharacter _ascharacter (+ (* (Math|Vector|Normalize (- (Transformation|GetActorLocation ObjectToApplyPushback) PushbackOriginLocation)) Strength) (Math|Vector|MakeVector 0.0 0.0 1e+01)) true true))