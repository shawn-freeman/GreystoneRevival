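; BP_Spell_Parent is a base projectile for spells that reports what it strikes and destroys itself on impact.
; The construction script sets up ProjectileMovement from the Speed and gravity scale variables, with rotation following velocity.
; When the collision box hits anything but the instigator, it calls the OnProjectileImpact dispatcher with that actor, then spawns impact particles and sound at the hit location.
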(event OnComponentHit(BoxCollision)
  (params (HitComponent :type Primitive%20Component%20Object%20Reference) (OtherActor :type Actor%20Object%20Reference) (OtherComp :type Primitive%20Component%20Object%20Reference) (NormalImpulse :type Vector :default "0, 0, 0") (Hit :type Hit%20Result%20Structure%20%28by%20ref%29))
  (bind _location (Collision|BreakHitResult Hit))
  (if (!= OtherActor (Game|GetInstigator))
    (Default|CallOnProjectileImpact OtherActor)
    (Effects|SpawnEmitteratLocation (Variables|Default|GetImpactFX) _location)
    (Audio|SpawnSoundatLocation (Variables|Default|GetImpactSoundFX) _location "0, 0, 0" 1.0 1.0 0.0 0 0)
    (Actor|DestroyActor)))

(fn ConstructionScript
  (Variables|/Script/Engine.ProjectileMovementComponent|SetInitialSpeed (Variables|Default|GetProjectileMovement) (Variables|Default|GetSpeed))
  (Variables|/Script/Engine.ProjectileMovementComponent|SetMaxSpeed (Variables|Default|GetProjectileMovement) (Variables|Default|GetSpeed))
  (Variables|/Script/Engine.ProjectileMovementComponent|SetbRotationFollowsVelocity (Variables|Default|GetProjectileMovement) true)
  (Variables|/Script/Engine.ProjectileMovementComponent|SetProjectileGravityScale (Variables|Default|GetProjectileMovement) (Variables|Default|GetProjectileGravityScale)))